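; BP_BadGuy is an enemy character that can die from damage or a high fall and awards score on death.
; Incoming damage reduces Health, triggering Die when it runs out.
; Tick detects fast falls, plays a looping falling animation and flags the enemy to die on landing.
; Die runs once, ragdolls the mesh, adds score through BP_GameMode, then after a delay destroys the actor and calls CallCheckEnemy.
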(event Custom|Die
  (bind _mesh (Variables|Character|GetMesh))
  ;[0.15 0.15 0.15 0.5] Enemy Death Script
  (Utilities|FlowControl|DoOnce false
    (:Completed
      (Collision|SetCollisionProfileName _mesh "Ragdoll" true :!class /Script/Engine.PrimitiveComponent)
      (Collision|SetCollisionEnabled _mesh "QueryAndPhysics")
      (Collision|SetCollisionProfileName (Variables|Collision|GetCapsuleComponent) "NoCollision" true :!class /Script/Engine.PrimitiveComponent)
      (Physics|SetSimulatePhysics (Variables|Character|GetMesh) true)
      (Default|AddScore (.AsBP%20Game%20Mode (Utilities|Casting|CastToBP_GameMode (Game|GetGameMode))) 250)
      (Utilities|FlowControl|Delay 5.0)
      (Actor|DestroyActor)
      (Default|CallCheckEnemy))))

(event EventDestroyed
  ;[0.15 0.15 0.15 0.5] Adding Score after death
)

(event EventTick
  (params (DeltaSeconds :type Float%20%28single-precision%29))
  (bind _charactermovement (Variables|Character|GetCharacterMovement))
  ;[0.15 0.15 0.15 0.5] Checking fall damage
  (if (and (AI|Components|NavMovement|IsFalling _charactermovement) (< (.z (Pawn|Components|CharacterMovement|GetLastUpdateVelocity _charactermovement)) -8e+02)) ; If the enemy is falling too fast it will trigger an istant death falling animation
    (Utilities|FlowControl|DoOnce false
      (:Completed
        (Components|Animation|PlayAnimation (Variables|Character|GetMesh) "/Game/Characters/Mannequins/Anims/Unarmed/Fall/Falling__1__Anim1.Falling__1__Anim1" true)
        (Components|Timeline|SetPlayRate (Variables|Character|GetMesh) 2.0)
        (Variables|Default|SetDieing%20to%20high%20fall true)))))

(event EventOnLanded
  (params (Hit :type Hit%20Result%20Structure%20%28by%20ref%29))
  ;[0.15 0.15 0.15 0.5] Checking fall damage
  (if (Variables|Default|GetDieing%20to%20high%20fall)
    (CallFunction|Die)))

(event Game|Damage|EventAnyDamage
  (params (Damage :type Float%20%28single-precision%29) (DamageType :type Damage%20Type%20Object%20Reference) (InstigatedBy :type Controller%20Object%20Reference) (DamageCauser :type Actor%20Object%20Reference))
  (Development|PrintString (Utilities|String|ToString(Float) Damage))
  ;[0.15 0.15 0.15 0.5] Adding Damage to health
  (if (> (Variables|Default|GetHealth) 0.0)
    (bind _output_get (Variables|Default|SetHealth (- (Variables|Default|GetHealth) Damage)))
    (if (<= _output_get 0.0)
      (CallFunction|Die))))

(fn ConstructionScript)