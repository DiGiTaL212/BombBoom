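; BP_Impact is a player-side explosive impact actor that detonates when its collision sphere hits something, then destroys itself.
; A zero-length multi-sphere trace finds actors within the explosion radius, sending an explode message to Explosive-tagged ones and applying damage to Enemy-tagged ones.
; It also spawns an explosion effect, applies a radial external-strain field to fracture Chaos geometry collections, and fires a force impulse.
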(event OnComponentHit(SphereCol)
  (params (HitComponent :type Primitive%20Component%20Object%20Reference) (OtherActor :type Actor%20Object%20Reference) (OtherComp :type Primitive%20Component%20Object%20Reference) (NormalImpulse :type Vector :default "0, 0, 0") (Hit :type Hit%20Result%20Structure%20%28by%20ref%29))
  (bind _output_get (Variables|Default|SetSelfLocation (Transformation|GetWorldLocation (Variables|Default|GetSphereCol))))
  (bind _outhits (Collision|MultiSphereTraceByChannel _output_get _output_get (Variables|Default|GetExplosion%20Radius) "TraceTypeQuery1" false 0 "None"))
  (for _array_element _outhits
    (if (Actor|ActorHasTag (.hitactor _array_element) "Explosive")
      (Class|BPIExplosive|Explode(Message) (.hitactor _array_element))
      (elif (Actor|ActorHasTag (.hitactor _array_element) "Enemy")
        (Game|Damage|ApplyDamage (.hitactor _array_element) 1e+02 (Game|GetPlayerController 0) self "/Script/Engine.DamageType"))))
  (Effects|SpawnEmitteratLocation "/Game/StarterContent/Particles/P_Explosion.P_Explosion" (Variables|Default|GetSelfLocation) "0, 0, 0" "4.000000,4.000000,4.000000")
  (Class|FieldSystemComponent|ApplyPhysicsField (Variables|Default|GetFieldSystem) true "Field_ExternalClusterStrain" 0 (Field|SetRadialFalloff (Variables|Default|GetRadialFalloff) 5e+08 0.0 1.0 0.0 (Variables|Default|GetExplosion%20Radius) (Variables|Default|GetSelfLocation) "Field_Falloff_Linear"))
  (Class|RadialForceComponent|FireImpulse (Variables|Default|GetExplosionForce))
  (Actor|DestroyActor))

(event EventBeginPlay)

(fn ConstructionScript)