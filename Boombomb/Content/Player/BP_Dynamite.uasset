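; Player dynamite actor that explodes after a short fuse starting on BeginPlay, then destroys itself.
; A multi-sphere trace at its collision sphere sends ExplodeMessage and ApplyDamage to hit actors tagged "Explosive", with distance-based damage falloff still unimplemented.
; It then spawns an explosion emitter, applies a linear radial-falloff external cluster strain field to fracture destructibles, and fires a radial force impulse.
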(event EventBeginPlay
  (Utilities|FlowControl|Delay 3.0)
  (bind _output_get (Variables|Default|SetSelfLocation (Transformation|GetWorldLocation (Variables|Default|GetSphereCol))))
  (bind _outhits (Collision|MultiSphereTraceByChannel _output_get _output_get (Variables|Default|GetExplosion%20Radius) "TraceTypeQuery1" false 0 "None"))
  (for _array_element _outhits
    (if (Actor|ActorHasTag (.hitactor _array_element) "Explosive")
      (Class|BPIExplosive|Explode(Message) (.hitactor _array_element))
      (Game|Damage|ApplyDamage (.hitactor _array_element) 0.0 0 0) ; This Needs to calculate the distance from the enemys within the explotion radius and apply the apropriate fall off damage value
    ))
  (Effects|SpawnEmitteratLocation "/Game/StarterContent/Particles/P_Explosion.P_Explosion" (Variables|Default|GetSelfLocation) "0, 0, 0" "6.000000,6.000000,6.000000")
  (Class|FieldSystemComponent|ApplyPhysicsField (Variables|Default|GetFieldSystem) true "Field_ExternalClusterStrain" 0 (Field|SetRadialFalloff (Variables|Default|GetRadialFalloff) 5e+08 0.0 1.0 0.0 (Variables|Default|GetExplosion%20Radius) (Variables|Default|GetSelfLocation) "Field_Falloff_Linear"))
  (Class|RadialForceComponent|FireImpulse (Variables|Default|GetExplosionForce))
  (Actor|DestroyActor))

(fn ConstructionScript)