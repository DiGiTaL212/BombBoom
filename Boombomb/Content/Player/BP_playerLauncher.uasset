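; Player launcher that fires dynamite or impact grenades with a slingshot-style mouse drag.
; Drag direction, with inverted yaw, and clamped length set rotation and strength, previewed by a debug-drawn predicted path.
; Release past a minimum drag spawns the selected projectile and sets its velocity.
; It also handles weapon selection, spring-arm camera drag, zoom and recentering, plus a pause widget gated by the game mode.
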(event Input|EnhancedActionEvents|EnhancedInputActionIA_MouseDown
  (params (ActionValue :type Boolean) (ElapsedSeconds :type Float%20%28double-precision%29) (TriggeredSeconds :type Float%20%28double-precision%29) (InputAction :type Input%20Action%20Object%20Reference :default "/Game/Player/Input/IA_MouseDown.IA_MouseDown"))
  (bind _self self)
  (bind _self_2 self)
  ;[0.15 0.15 0.15 0.5] Shooting & Aiming Funtion
  (:Triggered
    (bind _returnvalue (Class|WidgetLayoutLibrary|GetMousePositiononViewport))
    (Transformation|SetRelativeRotation (Variables|Default|GetArrow) (Math|Rotator|FindLookatRotation (Math|Vector|MakeVector 0.0 (.x _returnvalue) (.y (stale _output_get))) (Math|Vector|MakeVector 0.0 (.x (stale _output_get)) (.y _returnvalue))) false false)
    (Variables|ShootingValues|SetShootingDirection (Math|Rotator|MakeRotator (.Roll (Math|Rotator|BreakRotator (Math|Rotator|FindLookatRotation (Math|Vector|MakeVector 0.0 (.x _returnvalue) (.y (stale _output_get))) (Math|Vector|MakeVector 0.0 (.x (stale _output_get)) (.y _returnvalue))))) (.Pitch (Math|Rotator|BreakRotator (Math|Rotator|FindLookatRotation (Math|Vector|MakeVector 0.0 (.x _returnvalue) (.y (stale _output_get))) (Math|Vector|MakeVector 0.0 (.x (stale _output_get)) (.y _returnvalue))))) (* (.Yaw (Math|Rotator|BreakRotator (Math|Rotator|FindLookatRotation (Math|Vector|MakeVector 0.0 (.x _returnvalue) (.y (stale _output_get))) (Math|Vector|MakeVector 0.0 (.x (stale _output_get)) (.y _returnvalue))))) -1.0)))
    (Variables|ShootingValues|SetShootStrength (Math|Float|Lerp 0.0 2.5e+03 (/ (Math|Float|Clamp(Float) (Math|Vector|Distance2D(Vector) (Math|Vector2D|MakeVector2D (.x (stale _output_get)) (.y (stale _output_get))) (Math|Vector2D|MakeVector2D (.x _returnvalue) (.y _returnvalue))) 0.0 1e+02) 1e+02)))
    (if (> (/ (Math|Float|Clamp(Float) (Math|Vector|Distance2D(Vector) (Math|Vector2D|MakeVector2D (.x (stale _output_get)) (.y (stale _output_get))) (Math|Vector2D|MakeVector2D (.x _returnvalue) (.y _returnvalue))) 0.0 1e+02) 1e+02) 0.15)
      (Class|GameplayStatics|BlueprintPredictProjectilePathAdvanced (Utilities|Struct|MakePredictProjectilePathParams (Transformation|GetWorldLocation (Variables|Default|GetSphere)) (* (Math|Vector|GetForwardVector (Math|Rotator|MakeRotator (.Roll (Math|Rotator|BreakRotator (Math|Rotator|FindLookatRotation (Math|Vector|MakeVector 0.0 (.x _returnvalue) (.y (stale _output_get))) (Math|Vector|MakeVector 0.0 (.x (stale _output_get)) (.y _returnvalue))))) (.Pitch (Math|Rotator|BreakRotator (Math|Rotator|FindLookatRotation (Math|Vector|MakeVector 0.0 (.x _returnvalue) (.y (stale _output_get))) (Math|Vector|MakeVector 0.0 (.x (stale _output_get)) (.y _returnvalue))))) (* (.Yaw (Math|Rotator|BreakRotator (Math|Rotator|FindLookatRotation (Math|Vector|MakeVector 0.0 (.x _returnvalue) (.y (stale _output_get))) (Math|Vector|MakeVector 0.0 (.x (stale _output_get)) (.y _returnvalue))))) -1.0))) (Math|Float|Lerp 0.0 2.5e+03 (/ (Math|Float|Clamp(Float) (Math|Vector|Distance2D(Vector) (Math|Vector2D|MakeVector2D (.x (stale _output_get)) (.y (stale _output_get))) (Math|Vector2D|MakeVector2D (.x _returnvalue) (.y _returnvalue))) 0.0 1e+02) 1e+02))) false 0.0 1.0 true "ECC_WorldStatic" "ObjectTypeQuery1" 0 2e+01 0.0 "ForOneFrame" 1e+01 false))))
  (:Started
    (Utilities|FlowControl|Sequence
      (:then_0
        (bind _returnvalue_2 (UserInterface|CreateWidget "/Game/UI/WB_AimGuid.WB_AimGuid_C"))
        (Class|UserWidget|SetDesiredSizeinViewport _returnvalue_2 "(X=192.000000,Y=192.000000)")
        (UserInterface|Viewport|AddtoViewport _returnvalue_2 0))
      (:then_1
        (bind _returnvalue_3 (Class|WidgetLayoutLibrary|GetMousePositiononViewport))
        (bind _output_get (Variables|ShootingValues|SetLocation%20Start _returnvalue_3)))))
  (:Completed
    (if (> (/ (Math|Float|Clamp(Float) (Math|Vector|Distance2D(Vector) (Math|Vector2D|MakeVector2D (.x _output_get) (.y _output_get)) (Math|Vector2D|MakeVector2D (.x _returnvalue) (.y _returnvalue))) 0.0 1e+02) 1e+02) 0.15)
      (switch Utilities|FlowControl|Switch|SwitchonE_Throwable (Variables|Default|GetSelection)
        (:NewEnumerator0
          (bind _returnvalue_4 (Game|SpawnActorfromClass "/Game/Player/BP_Dynamite.BP_Dynamite_C" (Math|Transform|MakeTransform (Transformation|GetWorldLocation (Variables|Default|GetSphere)) (Variables|ShootingValues|GetShootingDirection) "1.000000,1.000000,1.000000") "Undefined" "MultiplyWithRoot" _self _self))
          (Variables|/Script/Engine.MovementComponent|SetVelocity (Variables|/Game/Player/BP_Dynamite.BP_Dynamite_C|GetProjectileMovement _returnvalue_4) (* (Transformation|GetActorForwardVector _returnvalue_4) (Variables|ShootingValues|GetShootStrength))))
        (:NewEnumerator1
          (bind _returnvalue_5 (Game|SpawnActorfromClass "/Game/Player/BP_Impact.BP_Impact_C" (Math|Transform|MakeTransform (Transformation|GetWorldLocation (Variables|Default|GetSphere)) (Variables|ShootingValues|GetShootingDirection) "1.000000,1.000000,1.000000") "Undefined" "MultiplyWithRoot" _self_2 _self_2))
          (Variables|/Script/Engine.MovementComponent|SetVelocity (Variables|/Game/Player/BP_Impact.BP_Impact_C|GetProjectileMovement _returnvalue_5) (* (Transformation|GetActorForwardVector _returnvalue_5) (Variables|ShootingValues|GetShootStrength))))))))

(event Input|EnhancedActionEvents|EnhancedInputActionIA_CameraMove
  (params (ActionValue :type Vector%202D%20Structure) (ElapsedSeconds :type Float%20%28double-precision%29) (TriggeredSeconds :type Float%20%28double-precision%29) (InputAction :type Input%20Action%20Object%20Reference :default "/Game/Player/Input/IA_CameraMove.IA_CameraMove"))
  ;[0.15 0.15 0.15 0.5] Camera Move Funtion
  (:Triggered
    (bind _returnvalue (Class|WidgetLayoutLibrary|GetMousePositiononViewport))
    (Transformation|SetRelativeLocation (Variables|Default|GetSpringArm) (+ (stale _output_get_2) (* (Math|Vector|GetForwardVector (Math|Rotator|FindLookatRotation (Math|Vector|MakeVector 0.0 (.x _returnvalue) (.y (stale _output_get))) (Math|Vector|MakeVector 0.0 (.x (stale _output_get)) (.y _returnvalue)))) (Math|Vector|Distance2D(Vector) (Math|Vector2D|MakeVector2D (.x (stale _output_get)) (.y (stale _output_get))) (Math|Vector2D|MakeVector2D (.x _returnvalue) (.y _returnvalue))))) true false))
  (:Started
    (bind _returnvalue_2 (Class|WidgetLayoutLibrary|GetMousePositiononViewport))
    (bind _output_get (Variables|CameraControls|SetCameraDragStartLocation _returnvalue_2))
    (bind _output_get_2 (Variables|CameraControls|SetCurrent%20Camera%20Relative%20Location (Variables|/Script/Engine.SceneComponent|GetRelativeLocation (Variables|Default|GetSpringArm))))))

(event Input|EnhancedActionEvents|EnhancedInputActionIA_CameraZoom
  (params (ActionValue :type Float%20%28double-precision%29) (ElapsedSeconds :type Float%20%28double-precision%29) (TriggeredSeconds :type Float%20%28double-precision%29) (InputAction :type Input%20Action%20Object%20Reference :default "/Game/Player/Input/IA_CameraZoom.IA_CameraZoom"))
  (bind _springarm (Variables|Default|GetSpringArm))
  ;[0.15 0.15 0.15 0.5] camera funtion
  (Variables|/Script/Engine.SpringArmComponent|SetTargetArmLength _springarm (Math|Float|Clamp(Float) (+ (* ActionValue -1e+02) (Variables|/Script/Engine.SpringArmComponent|GetTargetArmLength _springarm)) 6e+02 5e+03)))

(event Input|EnhancedActionEvents|EnhancedInputActionIA_RecenterCamera
  (params (ActionValue :type Boolean) (ElapsedSeconds :type Float%20%28double-precision%29) (TriggeredSeconds :type Float%20%28double-precision%29) (InputAction :type Input%20Action%20Object%20Reference :default "/Game/Player/Input/IA_RecenterCamera.IA_RecenterCamera"))
  ;[0.15 0.15 0.15 0.5] Recenter Camera
  (Transformation|SetRelativeLocation (Variables|Default|GetSpringArm) "0.000000,0.000000,90.000000" true false))

(event Input|EnhancedActionEvents|EnhancedInputActionIA_Pause
  (params (ActionValue :type Boolean) (ElapsedSeconds :type Float%20%28double-precision%29) (TriggeredSeconds :type Float%20%28double-precision%29) (InputAction :type Input%20Action%20Object%20Reference :default "/Game/Player/Input/IA_Pause.IA_Pause"))
  (bind _pausewidgitref (Variables|UI|GetPauseWidgitRef))
  ;[0.15 0.15 0.15 0.5] Pause Control
  (if (Variables|/Script/Engine.GameModeBase|GetbPauseable (Game|GetGameMode))
    (if (Game|IsGamePaused)
      (Widget|SetVisibility _pausewidgitref "Hidden")
      (Game|SetGamePaused false)
      (else
        (Widget|SetVisibility _pausewidgitref "Visible")
        (Game|SetGamePaused true)))))

(event Input|EnhancedActionEvents|EnhancedInputActionIA_Selection1
  (params (ActionValue :type Boolean) (ElapsedSeconds :type Float%20%28double-precision%29) (TriggeredSeconds :type Float%20%28double-precision%29) (InputAction :type Input%20Action%20Object%20Reference :default "/Game/Player/Input/IA_Selection1.IA_Selection1"))
  (Variables|Default|SetSelection "NewEnumerator0")
  (Components|StaticMesh|SetStaticMesh (Variables|Default|GetSelected) "/Game/Player/Assets/dynamite_1.dynamite_1"))

(event Input|EnhancedActionEvents|EnhancedInputActionIA_Selection2
  (params (ActionValue :type Boolean) (ElapsedSeconds :type Float%20%28double-precision%29) (TriggeredSeconds :type Float%20%28double-precision%29) (InputAction :type Input%20Action%20Object%20Reference :default "/Game/Player/Input/IA_Selection2.IA_Selection2"))
  (Variables|Default|SetSelection "NewEnumerator1")
  (Components|StaticMesh|SetStaticMesh (Variables|Default|GetSelected) "/Game/Player/Assets/Impact_grenade.Impact_grenade"))

(event EventBeginPlay
  ;[0.15 0.15 0.15 0.5] StartUp Setup
  (Variables|/Script/Engine.PlayerController|SetbShowMouseCursor (Game|GetPlayerController 0) true)
  (bind _returnvalue (UserInterface|CreateWidget "/Game/UI/WB_Pause.WB_Pause_C"))
  (Variables|UI|SetPauseWidgitRef _returnvalue)
  (UserInterface|Viewport|AddtoViewport _returnvalue 0))

(fn ConstructionScript)